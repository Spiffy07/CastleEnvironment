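; Game mode for a target game in which the player must score every BP_Target in the level before a countdown expires.
; BeginPlay sets the winning score from the target count, creates the WBP_UI HUD and starts a looping timer that decrements the countdown every tenth of a second.
; AddScore increments the score and refreshes the HUD.
; Reaching either limit calls EndGame, which shows WBP_EndScreen with the win/loss result and switches to UI-only input.
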(event Custom|AddScore
  (if (not (Variables|Default|GetIsGameOver))
    (Math|Integer|IncrementInt (Variables|Default|GetTargetScore)
      (:%20%20
        (Default|UpdateScore (Variables|Default|GetUI_Ref))
        (if (== (Variables|Default|GetTargetScore) (Variables|Default|GetMaxScore))
          (CallFunction|EndGame false))))))

(event Custom|DecrementTimer
  (bind _timer (Variables|Default|GetTimer))
  (if (not (Variables|Default|GetIsGameOver))
    (Math|Integer|DecrementInt _timer
      (:%20%20
        (Default|UpdateTimer (Variables|Default|GetUI_Ref))
        (if (<= _timer 0)
          (CallFunction|EndGame true))))))

(event EventBeginPlay
  (Input|SetInputModeGameOnly (Game|GetPlayerController 0) false)
  (bind _outactors (Actor|GetAllActorsOfClass "/Game/MyStuff/BP_Target.BP_Target_C"))
  (Variables|Default|SetMaxScore (Utilities|Array|Length _outactors))
  (Variables|Default|SetTargetScore 0)
  (bind _returnvalue (UserInterface|CreateWidget "/Game/MyStuff/WBP_UI.WBP_UI_C"))
  (bind _output_get (Variables|Default|SetUI_Ref _returnvalue))
  (UserInterface|Viewport|AddtoViewport _output_get 0)
  (Default|UpdateScore _output_get)
  (Utilities|Time|SetTimerbyEvent (delegate Custom|DecrementTimer) 0.1 true))

(fn ConstructionScript)

(fn EndGame
  (params (LostGame? :type Boolean))
  (bind _returnvalue (Game|GetPlayerController 0))
  (Variables|Default|SetIsGameOver true)
  (bind _returnvalue_2 (UserInterface|CreateWidget "/Game/MyStuff/WBP_EndScreen.WBP_EndScreen_C" 0 LostGame?))
  (UserInterface|Viewport|AddtoViewport _returnvalue_2 0)
  (Input|SetInputModeUIOnly _returnvalue _returnvalue_2 "DoNotLock" false)
  (Input|SetIgnoreMoveInput _returnvalue true)
  (Variables|/Script/Engine.PlayerController|SetbShowMouseCursor _returnvalue true))